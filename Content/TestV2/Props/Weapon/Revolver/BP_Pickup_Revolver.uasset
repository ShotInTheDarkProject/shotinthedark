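; Revolver pickup actor that gives the interacting character a handgun.
; On Interact, if the Interactor has no handgun yet, it sets HasHandgun and copies the pickup's ItemMesh static mesh onto the Interactor's Handgun component.
; It then plays a pickup sound at its location, destroys itself and calls SetEquipment on the Interactor to switch equipment.
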(event `/Game/TestV2/Blueprints/Interfaces/BPI_Interact.Interact`
  (params (Interactor :type "/Game/TestV2/Blueprints/Character/BP_FPHorrorCharacter Object Reference"))
  (if (not (`/Game/TestV2/Blueprints/Character/BP_FPHorrorCharacter.HasHandgun` Interactor))
    (set `/Game/TestV2/Blueprints/Character/BP_FPHorrorCharacter.HasHandgun` true Interactor)
    (`StaticMeshComponent.SetStaticMesh` (`/Game/TestV2/Blueprints/Character/BP_FPHorrorCharacter.Handgun` Interactor) (`StaticMeshComponent.StaticMesh` (`self.ItemMesh`)))
    (`GameplayStatics.PlaySoundAtLocation` (`self.PickupSound`) (`self.K2_GetActorLocation`) (struct) 1.0 1.0 0.0 null null null null)
    (`self.K2_DestroyActor`)
    (`/Game/TestV2/Blueprints/Character/BP_FPHorrorCharacter.SetEquipment` Interactor 1)))

(fn `UserConstructionScript`)