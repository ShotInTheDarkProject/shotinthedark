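; BP_DoorPunch is a weapon Blueprint that supplies the firing feedback for the Door Punch weapon.
; Its WeapFire event plays a sci-fi energy gun sound at the actor's location and a non-looping revolver fire animation on WeaponModel.
; It contains no hit, damage or projectile logic, and its construction script only calls the parent.
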(event `self.WeapFire`
  (`GameplayStatics.PlaySoundAtLocation` "/Game/TestV2/Audio/sci-fi-energy-gun-39409.sci-fi-energy-gun-39409" (`self.K2_GetActorLocation`) (struct) 1.0 1.0 0.0 null null null null)
  (`SkeletalMeshComponent.PlayAnimation` (`self.WeaponModel`) "/Game/TestV2/Weapons/RevolverPistol/ANI/AS_Weap_Revolver_Fire.AS_Weap_Revolver_Fire" false))

(fn `UserConstructionScript`
  (`parent.UserConstructionScript`))