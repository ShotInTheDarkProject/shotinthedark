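; Player-side component for interacting with BP_DoorMaster doors through traces cast from the camera.
; TraceForDoor sphere-traces and sends InteractMessage to the hit actor for manual interaction.
; InitializeTick runs two line-trace checks: OpenDoorHelper pushes physics-simulated doors with an impulse at the hit point while the player moves.
; DoorDetection auto-interacts with unlocked, inactive doors in a specific state when movement is fast enough, forcing them open.
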(fn `DoorDetection`
  (params (MovementComponent :type "MovementComponent Object Reference") (PlayerCamera :type "CameraComponent Object Reference") (TraceLength :type "Float (single-precision)" :default 50.0))
  (bind _returnvalue (`SceneComponent.K2_GetComponentLocation` PlayerCamera))
  (if (> (`KismetMathLibrary.VSize` (`MovementComponent.Velocity` MovementComponent)) 150.0)
    (bind (_outhit _returnvalue_2) (`KismetSystemLibrary.LineTraceSingle` _returnvalue (+ _returnvalue (* (`KismetMathLibrary.GetForwardVector` (`SceneComponent.K2_GetComponentRotation` PlayerCamera)) TraceLength)) "TraceTypeQuery1"))
    (if _returnvalue_2
      (bind _asbp_door_master (cast `/Game/TestV2/Blueprints/Interactables/Doors/BP_DoorMaster` (`.HitActor` (`GameplayStatics.BreakHitResult` _outhit))))
      (switch `/Game/TestV2/Blueprints/Enums/E_DoorLockTypes` (`/Game/TestV2/Blueprints/Interactables/Doors/BP_DoorMaster.DoorLockType` _asbp_door_master)
        (:`NewEnumerator0`
          (if (`|EnumEquality` (`/Game/TestV2/Blueprints/Interactables/Doors/BP_DoorMaster.DoorState` _asbp_door_master) "NewEnumerator0")
            (if (not (`/Game/TestV2/Blueprints/Interactables/Doors/BP_DoorMaster.StateActive` _asbp_door_master))
              (message `/Game/TestV2/Blueprints/Interfaces/BPI_Interact.Interact` _asbp_door_master))))))))

(fn `InitializeTick`
  (params (`Movement Component` :type "MovementComponent Object Reference") (`Player Camera` :type "CameraComponent Object Reference"))
  (`self.OpenDoorHelper` `Movement Component` `Player Camera` (`self.PushTraceLength`) (`self.PushStrength`))
  (`self.DoorDetection` `Movement Component` `Player Camera` (`self.ForceOpenTraceLength`)))

(fn `OpenDoorHelper`
  (params (`Movement Component` :type "MovementComponent Object Reference") (`Player Camera` :type "CameraComponent Object Reference") (`Trace Length` :type "Float (single-precision)" :default 80.0) (`Impulse Amount` :type "Float (double-precision)" :default 1000.0))
  (bind _returnvalue (`SceneComponent.K2_GetComponentLocation` `Player Camera`))
  (if (> (`KismetMathLibrary.VSize` (`MovementComponent.Velocity` `Movement Component`)) 0.0)
    (bind (_outhit _returnvalue_2) (`KismetSystemLibrary.LineTraceSingle` _returnvalue (+ _returnvalue (* (`KismetMathLibrary.GetForwardVector` (`SceneComponent.K2_GetComponentRotation` `Player Camera`)) `Trace Length`)) "TraceTypeQuery1" true))
    (if _returnvalue_2
      (bind (_bblockinghit _binitialoverlap _time _distance _location _impactpoint _normal _impactnormal _physmat _hitactor) (`GameplayStatics.BreakHitResult` _outhit))
      (bind _asbp_door_master (cast `/Game/TestV2/Blueprints/Interactables/Doors/BP_DoorMaster` _hitactor))
      (bind _door (`/Game/TestV2/Blueprints/Interactables/Doors/BP_DoorMaster.Door` _asbp_door_master))
      (if (`SceneComponent.IsSimulatingPhysics` _door "None")
        (`PrimitiveComponent.AddImpulseAtLocation` _door (* (`Actor.GetActorForwardVector` (`GameplayStatics.GetPlayerCharacter` 0)) `Impulse Amount`) _location "None")))))

(fn `TraceForDoor`
  (params (PlayerCamera :type "CameraComponent Object Reference") (`Trace Length` :type "Float (single-precision)" :default 180.0))
  (bind _returnvalue (`SceneComponent.K2_GetComponentLocation` PlayerCamera))
  (bind (_outhit _returnvalue_2) (`KismetSystemLibrary.SphereTraceSingle` _returnvalue (+ _returnvalue (* (`KismetMathLibrary.GetForwardVector` (`SceneComponent.K2_GetComponentRotation` PlayerCamera)) `Trace Length`)) 5.0 "TraceTypeQuery1"))
  (if _returnvalue_2
    (message `/Game/TestV2/Blueprints/Interfaces/BPI_Interact.Interact` (`.HitActor` (`GameplayStatics.BreakHitResult` _outhit)))))