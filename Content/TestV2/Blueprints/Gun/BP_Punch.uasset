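; BP_Punch is a gun-folder actor, apparently a punch projectile, that damages critter enemies and breaks doors on impact.
; Its sphere hit event acts only while the actor's speed is above a threshold.
; Critters take random ranged damage, multiplied tenfold on their Critical component, while BP_Door actors are destroyed outright.
; Fast impacts, barring failed casts, spawn an emitter and sound at the Bullet component, then destroy the actor.
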(event `self.Sphere.OnComponentHit`
  (params (HitComponent :type "PrimitiveComponent Object Reference") (OtherActor :type "Actor Object Reference") (OtherComp :type "PrimitiveComponent Object Reference") (NormalImpulse :type "Vector Structure") (Hit :type "HitResult Structure (by ref)"))
  (bind (_bblockinghit _binitialoverlap _time _distance _location _impactpoint _normal _impactnormal _physmat _hitactor _hitcomponent) (`GameplayStatics.BreakHitResult` Hit))
  (bind _returnvalue (`SceneComponent.K2_GetComponentLocation` (`self.Bullet`)))
  (if (> (`KismetMathLibrary.VSize` (`self.GetVelocity`)) 1000.0)
    (if (== (`GameplayStatics.GetObjectClass` OtherActor) "/Game/TestV2/Blueprints/Enemy/Critter/BP_Enemy_Critter.BP_Enemy_Critter_C")
      ;[0 0 0] Enemy (change damage 30~50)
      (bind _asbp_enemy_critter (cast `/Game/TestV2/Blueprints/Enemy/Critter/BP_Enemy_Critter` _hitactor))
      (if (== (`/Game/TestV2/Blueprints/Enemy/Critter/BP_Enemy_Critter.Critical` _asbp_enemy_critter) _hitcomponent)
        (`GameplayStatics.ApplyDamage` OtherActor (* (`KismetMathLibrary.RandomFloatInRange` (`self.DamageMin`) (`self.DamageMax`)) 10.0) null self "/Script/Engine.DamageType")
        (else
          (`GameplayStatics.ApplyDamage` OtherActor (`KismetMathLibrary.RandomFloatInRange` (`self.DamageMin`) (`self.DamageMax`)) null self "/Script/Engine.DamageType")))
      (elif (== (`GameplayStatics.GetObjectClass` OtherActor) "/Game/TestV2/Blueprints/QuickFix/BP_Door.BP_Door_C")
        (bind _asbp_door (cast `/Game/TestV2/Blueprints/QuickFix/BP_Door` OtherActor))
        (`self.K2_DestroyActor` _asbp_door)))
    (`GameplayStatics.SpawnEmitterAtLocation` null _returnvalue)
    (`GameplayStatics.PlaySoundAtLocation` null _returnvalue (struct) 1.0 1.0 0.0 null null null null)
    (`self.K2_DestroyActor`)))

(fn `UserConstructionScript`)