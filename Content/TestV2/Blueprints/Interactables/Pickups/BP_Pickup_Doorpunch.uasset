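; Interactable pickup that gives the player the Doorpunch equipment.
; On Interact it finds the nearest BP_FPHorrorCharacter and, if that character lacks the Doorpunch, sets its flag, plays a pickup sound, destroys itself and switches the character's equipment to it.
; The sphere overlap events are empty, leaving the PickupPrompt show and hide calls disconnected.
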(event `self.Interact`
  (params (Interactor :type "/Game/TestV2/Blueprints/Character/BP_FPHorrorCharacter Object Reference"))
  (bind _outactors (`GameplayStatics.GetAllActorsOfClass` "/Game/TestV2/Blueprints/Character/BP_FPHorrorCharacter.BP_FPHorrorCharacter_C"))
  (bind _asbp_fphorror_character (cast `/Game/TestV2/Blueprints/Character/BP_FPHorrorCharacter` (`.ReturnValue` (`GameplayStatics.FindNearestActor` (`self.K2_GetActorLocation`) _outactors))))
  (if (not (`/Game/TestV2/Blueprints/Character/BP_FPHorrorCharacter.HasDoorpunch` _asbp_fphorror_character))
    (set `/Game/TestV2/Blueprints/Character/BP_FPHorrorCharacter.HasDoorpunch` true _asbp_fphorror_character)
    (`GameplayStatics.PlaySoundAtLocation` (`self.PickupSound`) (`self.K2_GetActorLocation`) (struct) 1.0 1.0 0.0 null null null null)
    (`self.K2_DestroyActor`)
    (`/Game/TestV2/Blueprints/Character/BP_FPHorrorCharacter.SetEquipment` _asbp_fphorror_character 2)))

(event `self.Sphere.OnComponentBeginOverlap`
  (params (OverlappedComponent :type "PrimitiveComponent Object Reference") (OtherActor :type "Actor Object Reference") (OtherComp :type "PrimitiveComponent Object Reference") (OtherBodyIndex :type Integer) (bFromSweep :type Boolean) (SweepResult :type "HitResult Structure (by ref)")))

(event `self.Sphere.OnComponentEndOverlap`
  (params (OverlappedComponent :type "PrimitiveComponent Object Reference") (OtherActor :type "Actor Object Reference") (OtherComp :type "PrimitiveComponent Object Reference") (OtherBodyIndex :type Integer)))

(fn `UserConstructionScript`
  (`parent.UserConstructionScript`))