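; BP_Pickup_Ammo is an interactable pickup that gives the player handgun ammunition.
; On Interact, it adds its Bullets amount to the interactor's HandgunAmmo and refreshes that interactor's ammo counter.
; It then plays the pickup sound at its location and destroys itself.
; The construction script only calls the parent's version.
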(event `self.Interact`
  (params (Interactor :type "/Game/TestV2/Blueprints/Character/BP_FPHorrorCharacter Object Reference"))
  (set `/Game/TestV2/Blueprints/Character/BP_FPHorrorCharacter.HandgunAmmo` (+ (`/Game/TestV2/Blueprints/Character/BP_FPHorrorCharacter.HandgunAmmo` Interactor) (`self.Bullets`)) Interactor)
  (`/Game/TestV2/Blueprints/Character/BP_FPHorrorCharacter.UpdateAmmoCounter` Interactor)
  (`GameplayStatics.PlaySoundAtLocation` (`self.PickupSound`) (`self.K2_GetActorLocation`) (struct) 1.0 1.0 0.0 null null null null)
  (`self.K2_DestroyActor`))

(fn `UserConstructionScript`
  (`parent.UserConstructionScript`))