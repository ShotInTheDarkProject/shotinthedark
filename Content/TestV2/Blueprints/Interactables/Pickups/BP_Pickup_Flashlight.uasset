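; Flashlight pickup actor that grants the flashlight to the horror first-person player character when interacted with.
; On Interact, it casts player 0 to BP_FPHorrorCharacter, sets HasFlashlight and copies its ItemMesh static mesh onto the character's Flashlight component.
; It then plays the pickup sound at its location and destroys itself.
; The construction script only calls the parent's.
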(event `/Game/TestV2/Blueprints/Interfaces/BPI_Interact.Interact`
  (bind _asbp_fphorror_character (cast `/Game/TestV2/Blueprints/Character/BP_FPHorrorCharacter` (`GameplayStatics.GetPlayerCharacter` 0)))
  (set `/Game/TestV2/Blueprints/Character/BP_FPHorrorCharacter.HasFlashlight` true _asbp_fphorror_character)
  ;[1 0 0 0.296] 注释
  (`StaticMeshComponent.SetStaticMesh` (`/Game/TestV2/Blueprints/Character/BP_FPHorrorCharacter.Flashlight` _asbp_fphorror_character) (`StaticMeshComponent.StaticMesh` (`self.ItemMesh`)))
  (`GameplayStatics.PlaySoundAtLocation` (`self.PickupSound`) (`self.K2_GetActorLocation`) (struct) 1.0 1.0 0.0 null null null null)
  (`self.K2_DestroyActor`))

(fn `UserConstructionScript`
  (`parent.UserConstructionScript`))