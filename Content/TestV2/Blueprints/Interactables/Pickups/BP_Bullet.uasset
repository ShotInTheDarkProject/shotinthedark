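; BP_Bullet is a projectile actor that damages BP_Enemy_Critter enemies and destroys itself after DespawnTime.
; On a hit above a speed threshold, it applies random damage between DamageMin and DamageMax, multiplied tenfold when the struck component is the critter's Critical component, then destroys itself.
; Slower hits and hits on other actor classes do nothing.
; An unconnected tag-based damage branch remains in the graph.
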(event `self.ReceiveBeginPlay`
  (`KismetSystemLibrary.Delay` (`self.DespawnTime`))
  (`self.K2_DestroyActor`))

(event `self.ReceiveHit`
  (params (MyComp :type "PrimitiveComponent Object Reference") (Other :type "Actor Object Reference") (OtherComp :type "PrimitiveComponent Object Reference") (bSelfMoved :type Boolean) (HitLocation :type "Vector Structure") (HitNormal :type "Vector Structure") (NormalImpulse :type "Vector Structure") (Hit :type "HitResult Structure (by ref)"))
  (bind (_bblockinghit _binitialoverlap _time _distance _location _impactpoint _normal _impactnormal _physmat _hitactor _hitcomponent) (`GameplayStatics.BreakHitResult` Hit))
  (if (> (`KismetMathLibrary.VSize` (`self.GetVelocity`)) 1000.0)
    (if (== (`GameplayStatics.GetObjectClass` Other) "/Game/TestV2/Blueprints/Enemy/Critter/BP_Enemy_Critter.BP_Enemy_Critter_C")
      (bind _asbp_enemy_critter (cast `/Game/TestV2/Blueprints/Enemy/Critter/BP_Enemy_Critter` _hitactor))
      (if (== (`/Game/TestV2/Blueprints/Enemy/Critter/BP_Enemy_Critter.Critical` _asbp_enemy_critter) _hitcomponent)
        (`GameplayStatics.ApplyDamage` Other (* (`KismetMathLibrary.RandomFloatInRange` (`self.DamageMin`) (`self.DamageMax`)) 10.0) null self "/Script/Engine.DamageType")
        (`self.K2_DestroyActor`)
        (else
          (`GameplayStatics.ApplyDamage` Other (`KismetMathLibrary.RandomFloatInRange` (`self.DamageMin`) (`self.DamageMax`)) null self "/Script/Engine.DamageType")
          (`self.K2_DestroyActor`))))))

(fn `UserConstructionScript`)