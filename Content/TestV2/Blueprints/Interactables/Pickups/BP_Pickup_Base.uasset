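; BP_Pickup_Base is a base interactable pickup that shows an in-world "Press E / X to Pick Up" prompt.
; BeginPlay sets the keyboard and controller prompt text on its W_ButtonContextInteract widget.
; ShowButtonContext moves the widget component to the ButtonContextLocation marker, rotates it to face the given player and toggles its visibility.
; The Interact event is empty, so this Blueprint itself implements no pickup behavior.
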(event `/Game/TestV2/Blueprints/Interfaces/BPI_Interact.Interact`
  (params (Interactor :type "/Game/TestV2/Blueprints/Character/BP_FPHorrorCharacter Object Reference")))

(event `self.ReceiveBeginPlay`
  (bind _asw_button_context_interact (cast `/Game/TestV2/Widgets/W_ButtonContextInteract` (`WidgetComponent.GetWidget` (`self.ButtonContextWidget`))))
  (`/Game/TestV2/Widgets/W_ButtonContextInteract.SetPromptText` _asw_button_context_interact "Press" "E" "X" "to Pick Up"))

(fn `ShowButtonContext`
  (params (Visible :type Boolean) (Player :type "/Game/TestV2/Blueprints/Character/BP_FPHorrorCharacter Object Reference"))
  (bind _buttoncontextwidget (`self.ButtonContextWidget`))
  (`SceneComponent.K2_SetWorldLocation` _buttoncontextwidget (`SceneComponent.K2_GetComponentLocation` (`self.ButtonContextLocation`)) false false)
  (`SceneComponent.K2_SetWorldRotation` _buttoncontextwidget (`KismetMathLibrary.FindLookAtRotation` (`SceneComponent.K2_GetComponentLocation` _buttoncontextwidget) (`SceneComponent.K2_GetComponentLocation` (`Actor.RootComponent` Player))) false false)
  (`SceneComponent.SetVisibility` _buttoncontextwidget Visible false))

(fn `UserConstructionScript`)