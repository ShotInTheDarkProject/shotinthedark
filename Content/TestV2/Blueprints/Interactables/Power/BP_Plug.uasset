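; BP_Plug is a carryable plug interactable that attaches to an outlet and relays power to it.
; Connect stores the outlet, drops the plug and turns off mesh physics.
; Disconnect clears the connection, restores physics and passes a valid interactor to Interact.
; PowerConnection stores the incoming power value and forwards it to the connected BP_Outlet through PowerConnections.
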(fn `Connect`
  (params (Outlet :type "/Game/TestV2/Blueprints/Interactables/Power/BP_Outlet Object Reference"))
  (set `self.Connection` Outlet)
  (`self.Drop`)
  (`PrimitiveComponent.SetSimulatePhysics` (`self.Mesh`) false))

(fn `Disconnect`
  (params (Interactor :type "/Game/TestV2/Blueprints/Character/BP_FPHorrorCharacter Object Reference"))
  (set `self.Connection` null)
  (`PrimitiveComponent.SetSimulatePhysics` (`self.Mesh`) true)
  (`/Engine/EditorBlueprintResources/StandardMacros.IsValid` Interactor
    (:`Is Valid`
      (`self.Interact` Interactor))))

(fn `PowerConnection`
  (params (Input :type Boolean))
  (bind _output_get (set `self.Power` Input))
  (bind _asbp_outlet (cast `/Game/TestV2/Blueprints/Interactables/Power/BP_Outlet` (`self.Connection`)))
  (`/Game/TestV2/Blueprints/Interactables/Power/BP_Outlet.PowerConnections` _asbp_outlet _output_get))

(fn `UserConstructionScript`
  (`parent.UserConstructionScript`))