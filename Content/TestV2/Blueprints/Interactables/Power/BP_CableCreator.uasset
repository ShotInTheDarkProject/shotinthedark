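; BP_CableCreator is a power interactable that spawns a plug and cable and passes its Power value to that plug.
; On BeginPlay it spawns BP_Plug at PlugPosition, registers itself as its Source, then spawns BP_Cable there with the cable end attached to the plug.
; PowerConnection stores Power and forwards it to the plug, starting with the initial value.
; Tick draws Power as debug text at the actor's location.
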(event `self.ReceiveBeginPlay`
  (bind _returnvalue (`|SpawnActorFromClass` "/Game/TestV2/Blueprints/Interactables/Power/BP_Plug.BP_Plug_C" (`KismetMathLibrary.Conv_VectorToTransform` (`SceneComponent.K2_GetComponentLocation` (`self.PlugPosition`))) "Undefined" "MultiplyWithRoot" null null))
  (set `/Game/TestV2/Blueprints/Interactables/Power/BP_Plug.Source` self _returnvalue)
  (bind _output_get (set `self.Plug` _returnvalue))
  (bind _returnvalue_2 (`|SpawnActorFromClass` "/Game/TestV2/Blueprints/Interactables/Power/BP_Cable.BP_Cable_C" (`KismetMathLibrary.Conv_VectorToTransform` (`self.K2_GetActorLocation` _output_get)) "Undefined" "MultiplyWithRoot" null null))
  (`CableComponent.SetAttachEndTo` (`CableActor.CableComponent` _returnvalue_2) (`self.Plug`) "None" "None")
  (`self.PowerConnection` (`self.Power`)))

(event `self.ReceiveTick`
  (params (DeltaSeconds :type "Float (single-precision)"))
  (`KismetSystemLibrary.DrawDebugString` (`self.K2_GetActorLocation`) (`KismetStringLibrary.Conv_BoolToString` (`self.Power`)) null (struct :`R` 1.0 :`G` 0.681906 :`A` 1.0)))

(fn `PowerConnection`
  (params (Input :type Boolean))
  (bind _output_get (set `self.Power` Input))
  (`/Game/TestV2/Blueprints/Interactables/Power/BP_Plug.PowerConnection` (`self.Plug`) _output_get))

(fn `UserConstructionScript`)