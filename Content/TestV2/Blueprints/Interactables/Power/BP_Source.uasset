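; BP_Source is a power source interactable that passes its powered state and color type to a connected plug.
; On BeginPlay it colors its outlet by type, optionally spawns a BP_Plug linked as its output with a BP_CablePower attached to it, then applies its initial power state.
; Switch swaps the light's glow material and forwards the state to the output, while SetType picks a red, green or blue outlet material.
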(event `self.ReceiveBeginPlay`
  (`|ExecutionSequence`
    (:`then_0`
      (`self.SetType` (`self.Type`)))
    (:`then_1`
      (if (`self.SpawnPlug`)
        (bind _returnvalue (`|SpawnActorFromClass` "/Game/TestV2/Blueprints/Interactables/Power/BP_Plug.BP_Plug_C" (`SceneComponent.K2_GetComponentToWorld` (`self.PlugSpawn`)) "AlwaysSpawn" "MultiplyWithRoot" null null))
        (set `/Game/TestV2/Blueprints/Interactables/Power/BP_Plug.Input` self _returnvalue)
        (set `self.Output` _returnvalue)
        (`/Game/TestV2/Blueprints/Interactables/Power/BP_Plug.SetType` _returnvalue (`self.Type`))
        (bind _returnvalue_2 (`|SpawnActorFromClass` "/Game/TestV2/Blueprints/Interactables/Power/BP_CablePower.BP_CablePower_C" (`SceneComponent.K2_GetComponentToWorld` (`self.CableSpawn`)) "AlwaysSpawn" "MultiplyWithRoot" self null))
        (`CableComponent.SetAttachEndToComponent` (`CableActor.CableComponent` _returnvalue_2) (`/Game/TestV2/Blueprints/Interactables/Power/BP_Plug.CableAttach` (`self.Output`)) "None")))
    (:`then_2`
      (`self.Switch` (`self.Powered`)))))

(fn `SetType`
  (params (Type :type Integer))
  (bind _output_get (set `self.Type` Type))
  (if (== _output_get 0)
    (`PrimitiveComponent.SetMaterial` (`self.Outlet`) 0 "/Game/TestV2/Props/EnvironmentModule/Plugs_Inlet/Materials/Plug_Red.Plug_Red")
    (elif (== _output_get 1)
      (`PrimitiveComponent.SetMaterial` (`self.Outlet`) 0 "/Game/TestV2/Props/EnvironmentModule/Plugs_Inlet/Materials/Plug_Green.Plug_Green")
      (elif (== _output_get 2)
        (`PrimitiveComponent.SetMaterial` (`self.Outlet`) 0 "/Game/TestV2/Props/EnvironmentModule/Plugs_Inlet/Materials/Plug_Blue.Plug_Blue")))))

(fn `Switch`
  (params (Powered :type Boolean))
  (bind _output (`self.Output`))
  (bind _light (`self.Light`))
  (bind _output_get (set `self.Powered` Powered))
  (if _output_get
    (`PrimitiveComponent.SetMaterial` _light 0 "/Game/TestV2/Materials/M_GlowPowered.M_GlowPowered")
    (else
      (`PrimitiveComponent.SetMaterial` _light 0 "/Game/TestV2/Materials/M_GlowUnpowered.M_GlowUnpowered")))
  (if (`KismetSystemLibrary.IsValid` _output)
    (`/Game/TestV2/Blueprints/Interactables/Power/BP_Plug.Switch` _output (`self.Powered`))))

(fn `UserConstructionScript`)