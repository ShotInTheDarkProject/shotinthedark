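; BP_Outlet is an interactable power socket that passes power from a connected BP_Plug to the actors in its Powers list.
; An overlapping plug connects and snaps to the Arrow, unless its Source is already in that list.
; PowerConnections forwards the power state to cable creators and opens or closes doors.
; Interacting disconnects the plug and cuts power, while Tick draws the power state as debug text.
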(event `/Game/TestV2/Blueprints/Interfaces/BPI_Interact.Interact`
  (params (Interactor :type "/Game/TestV2/Blueprints/Character/BP_FPHorrorCharacter Object Reference"))
  (bind _connection (`self.Connection`))
  (`/Engine/EditorBlueprintResources/StandardMacros.IsValid` _connection
    (:`Is Valid`
      (`/Game/TestV2/Blueprints/Interactables/Power/BP_Plug.Disconnect` _connection Interactor)
      (set `self.Connection` null)
      (`self.PowerConnections` false))))

(event `self.ReceiveActorBeginOverlap`
  (params (OtherActor :type "Actor Object Reference"))
  (bind _arrow (`self.Arrow`))
  (`/Engine/EditorBlueprintResources/StandardMacros.IsValid` (`self.Connection`)
    (:`Is Not Valid`
      (if (== (`GameplayStatics.GetObjectClass` OtherActor) "/Game/TestV2/Blueprints/Interactables/Power/BP_Plug.BP_Plug_C")
        (bind _asbp_plug (cast `/Game/TestV2/Blueprints/Interactables/Power/BP_Plug` OtherActor))
        (if (not (`KismetArrayLibrary.Array_Contains` (`self.Powers`) (`/Game/TestV2/Blueprints/Interactables/Power/BP_Plug.Source` _asbp_plug)))
          (set `self.Connection` _asbp_plug)
          (`/Game/TestV2/Blueprints/Interactables/Power/BP_Plug.Connect` (`self.Connection`) self)
          (`self.K2_SetActorLocationAndRotation` OtherActor (`SceneComponent.K2_GetComponentLocation` _arrow) (`SceneComponent.K2_GetComponentRotation` _arrow) false true)
          (`self.PowerConnections` (`/Game/TestV2/Blueprints/Interactables/Power/BP_Plug.Power` (`self.Connection`))))))))

(event `self.ReceiveTick`
  (params (DeltaSeconds :type "Float (single-precision)"))
  (`KismetSystemLibrary.DrawDebugString` (`self.K2_GetActorLocation`) (`KismetStringLibrary.Conv_BoolToString` (`self.Power`)) null (struct :`R` 1.0 :`G` 0.681906 :`A` 1.0)))

(fn `PowerConnections`
  (params (Input :type Boolean))
  (bind _output_get (set `self.Power` Input))
  (for _array_element (`self.Powers`)
    (bind _asbp_cable_creator (cast `/Game/TestV2/Blueprints/Interactables/Power/BP_CableCreator` _array_element)
      (:`then`
        (`/Game/TestV2/Blueprints/Interactables/Power/BP_CableCreator.PowerConnection` _asbp_cable_creator _output_get))
      (:`CastFailed`
        (bind _asbp_door (cast `/Game/TestV2/Blueprints/QuickFix/BP_Door` _array_element))
        (if _output_get
          (`/Game/TestV2/Blueprints/QuickFix/BP_Door.Open` _asbp_door)
          (else
            (`/Game/TestV2/Blueprints/QuickFix/BP_Door.Close` _asbp_door)))))))

(fn `UserConstructionScript`)