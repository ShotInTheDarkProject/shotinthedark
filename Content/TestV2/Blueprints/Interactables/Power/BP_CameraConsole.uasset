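; BP_CameraConsole is a powered interactable console that displays a live feed from a linked Camera on a widget screen.
; On BeginPlay it sets the W_CameraConsole screen brush to the camera's FeedMaterial, calling parent BeginPlay only if a camera is set and the cast succeeds.
; The Switch override calls the parent, then shows or hides the widget component with the powered state when a camera is assigned.
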(event `self.ReceiveBeginPlay`
  (bind _camera (`self.Camera`))
  (`/Engine/EditorBlueprintResources/StandardMacros.IsValid` _camera
    (:`Is Valid`
      (bind _asw_camera_console (cast `/Game/TestV2/Widgets/W_CameraConsole` (`WidgetComponent.GetWidget` (`self.WC_CameraConsole`))))
      (bind _output_get (set `self.Widget` _asw_camera_console))
      (`Image.SetBrushFromMaterial` (`/Game/TestV2/Widgets/W_CameraConsole.Screen` _output_get) (`/Game/TestV2/Blueprints/Interactables/Power/BP_SecurityCamera.FeedMaterial` _camera))
      (`parent.ReceiveBeginPlay`))))

(fn `Switch`
  (params (Powered :type Boolean))
  (`parent.Switch` Powered)
  (`/Engine/EditorBlueprintResources/StandardMacros.IsValid` (`self.Camera`)
    (:`Is Valid`
      (`SceneComponent.SetVisibility` (`self.WC_CameraConsole`) (`local.Powered`) true))))

(fn `UserConstructionScript`
  (`parent.UserConstructionScript`))