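; BP_Generator is an interactable power generator that can show rails and feed power through an outlet.
; On BeginPlay it optionally makes its Rails visible and spawns a BP_Source actor at the OutletSpawn point, storing it as Output.
; Its Switch function stores the Powered state and passes it on to that Output, which is also called right after spawning to apply the initial state.
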(event `self.ReceiveBeginPlay`
  (`|ExecutionSequence`
    (:`then_0`
      (if (`self.SpawnRails`)
        (`SceneComponent.SetVisibility` (`self.Rails`) true true)))
    (:`then_1`
      (if (`self.SpawnOutlet`)
        (bind _returnvalue (`|SpawnActorFromClass` "/Game/TestV2/Blueprints/Interactables/Power/BP_Source.BP_Source_C" (`SceneComponent.K2_GetComponentToWorld` (`self.OutletSpawn`)) "AlwaysSpawn" "MultiplyWithRoot" null null))
        (set `self.Output` _returnvalue)
        (`self.Switch` (`self.Powered`))))))

(fn `Switch`
  (params (Powered :type Boolean))
  (bind _output_get (set `self.Powered` Powered))
  (`/Game/TestV2/Blueprints/Interactables/Power/BP_Source.Switch` (`self.Output`) _output_get))

(fn `UserConstructionScript`)