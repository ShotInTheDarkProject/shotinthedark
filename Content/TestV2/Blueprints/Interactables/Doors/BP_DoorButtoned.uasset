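; BP_DoorButtoned is a door Blueprint that spawns its own BP_ButtonDoor buttons on BeginPlay.
; SpawnButton spawns a button at a marker's transform, adds the door to its OutputTo list and attaches it to a door component.
; ButtonFront gates a button on Right; ButtonBack, checked only after that, gates one on Left.
; Parent BeginPlay runs only when both flags are true.
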(event `SpawnButton`
  (params (SpawnComponent :type "ArrowComponent Object Reference") (DoorComponent :type "MeshComponent Object Reference"))
  (bind _returnvalue (`|SpawnActorFromClass` "/Game/TestV2/Blueprints/Interactables/Doors/BP_ButtonDoor.BP_ButtonDoor_C" (`SceneComponent.K2_GetComponentToWorld` SpawnComponent) "AlwaysSpawn" "MultiplyWithRoot" null null))
  (`KismetArrayLibrary.Array_Add` (`/Game/TestV2/Blueprints/QuickFix/BP_ClickButton.Output to:` _returnvalue) self)
  (`self.K2_AttachToComponent` _returnvalue DoorComponent "None" "KeepWorld" "KeepWorld" "KeepWorld" true))

(event `self.ReceiveBeginPlay`
  (if (`self.ButtonFront`)
    (`self.SpawnButton` (`self.ButtonSpawn1`) (`self.Right`))
    (if (`self.ButtonBack`)
      (`self.SpawnButton` (`self.ButtonSpawn2`) (`self.Left`))
      (`parent.ReceiveBeginPlay`))))

(fn `UserConstructionScript`
  (`parent.UserConstructionScript`))