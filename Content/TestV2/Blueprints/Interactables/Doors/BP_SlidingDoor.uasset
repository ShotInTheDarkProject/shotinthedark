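; Sliding door that the player opens and closes with the left mouse button while inside its trigger range.
; Overlap events track the player; the box is detached on BeginPlay, keeping the trigger still as the root moves.
; A FlipFlop plays or reverses a timeline that slides the root along world X by a set amount.
; VInterpTo serves as a lerp, taking the timeline track as DeltaTime.
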(event `self.ReceiveActorBeginOverlap`
  (params (OtherActor :type "Actor Object Reference"))
  (if (== OtherActor (`GameplayStatics.GetPlayerCharacter` 0))
    (set `self.IsPlayerInRange` true)))

(event `self.ReceiveActorEndOverlap`
  (params (OtherActor :type "Actor Object Reference"))
  (if (== null (`GameplayStatics.GetPlayerCharacter` 0))
    (set `self.IsPlayerInRange` false)))

(event `self.ReceiveBeginPlay`
  (`SceneComponent.K2_DetachFromComponent` (`self.Box`) "KeepRelative" "KeepWorld" "KeepWorld" true)
  (bind _output_get (set `self.InitialDoorPosition` (`SceneComponent.K2_GetComponentLocation` (`self.DefaultSceneRoot`))))
  (set `self.EndDoorPosition` (`KismetMathLibrary.MakeVector` (+ (.x _output_get) (`self.DoorSlidingAmount`)) (.y _output_get) (.z _output_get))))

(event `Key|LeftMouseButton`
  (params (Key :type "Key Structure"))
  (:`Pressed`
    (if (`self.IsPlayerInRange`)
      (`/Engine/EditorBlueprintResources/StandardMacros.FlipFlop`
        (:`A`
          (bind (_direction _sliding) (`Timeline|SlidingDoor` :!label _label)
            (:`Update`
              (`SceneComponent.K2_SetWorldLocation` (`self.DefaultSceneRoot`) (`KismetMathLibrary.VInterpTo` (`self.InitialDoorPosition`) (`self.EndDoorPosition`) _sliding 1.0) false false))))
        (:`B`
          (goto _label :!via `Reverse`))))))

(fn `UserConstructionScript`)