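; Master interactable door that opens away from the player, can be locked or forced, and closes when the player leaves its trigger.
; Interact cycles Closed, Part Open and Open through timeline rotations, while locked doors jiggle with a sound.
; Part Open hands the door to physics, with a delay loop polling yaw to auto-open past a threshold and driving velocity-based sound.
; Leaving physics reattaches the door to its frame before the timeline resumes.
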(event `ActivatePhysicsSound`
  ;[0.01 0.01 0.01] HandlePhysicsSounds
  (`AudioComponent.FadeIn` (`self.PhysicsSoundComponent`) 0.1 1.0 0.0 "Linear"))

(event `self.ReceiveBeginPlay`
  ;[0.01 0.01 0.01] Create Physics Sound
  (bind _returnvalue (`AddComponent|NODE_AddAudioComponent-1` :`bManualAttachment` true :`RelativeTransform` (`self.GetTransform`)))
  (bind _output_get (set `self.PhysicsSoundComponent` _returnvalue))
  (`AudioComponent.SetSound` _output_get (`self.PhysicsSound`))
  (`AudioComponent.FadeOut` _output_get 0.0 0.0 "Linear"))

(event `ClearPhysicsSound`
  ;[0.01 0.01 0.01] HandlePhysicsSounds
  (`AudioComponent.FadeOut` (`self.PhysicsSoundComponent`) 0.1 0.0 "Linear")
  (`self.ResetPhysics Sound`))

(event `/Game/TestV2/Blueprints/Interfaces/BPI_Interact.Interact`
  ;[0.01 0.01 0.01] Trigger Interact With Door
  (set `self.DoorDirection` (`self.CalculateOpenDirection`))
  (switch `/Game/TestV2/Blueprints/Enums/E_DoorLockTypes` (`self.DoorLockType`)
    (:`NewEnumerator0`
      (bind _door_state (`self.UpdateDoorState`))
      (switch `/Game/TestV2/Blueprints/Enums/E_DoorStates` _door_state
        (:`NewEnumerator1`
          (`KismetSystemLibrary.Delay` 0.1)
          (`self.StopDoor_TL`)
          (`PrimitiveComponent.SetSimulatePhysics` (`self.Door`) true)
          (`self.CheckDoorRotation`))))
    (:`NewEnumerator1`
      (`self.LockedEvent`))))

(event `RotateDoor`
  (params (`Target Rotation` :type "Float (double-precision)"))
  ;[0.01 0.01 0.01] Rotate Door
  (set `self.StateActive` true)
  (`|ExecutionSequence`
    (:`then_0`
      (bind (_direction _alpha) (`Timeline|Door_TL` :!via `PlayFromStart` :!label _label)
        (:`Update`
          (`SceneComponent.K2_SetRelativeRotation` (`self.Door`) (`KismetMathLibrary.RLerp` (`SceneComponent.RelativeRotation` (`self.Door`)) (`KismetMathLibrary.MakeRotator` 0.0 0.0 (* `Target Rotation` (`self.DoorDirection`))) _alpha) false false))))
    (:`then_1`
      (`KismetSystemLibrary.RetriggerableDelay` 0.8)
      (set `self.StateActive` false))))

(event `StopDoor_TL`
  ;[0.01 0.01 0.01] Rotate Door
  (set `self.StateActive` false)
  (goto _label :!via `Stop`))

(event `CheckDoorRotation`
  (bind _degree (`self.CalculatePhysicsDoorDegree`))
  (bind _autoopenangle (`self.AutoOpenAngle`))
  ;[0.01 0.01 0.01] Check if Door is open past designated degrees.
  (`self.TriggerPhysicsSound`)
  (if (`SceneComponent.IsSimulatingPhysics` (`self.Door`) "None")
    (if (> _degree 0.0)
      (if (> _degree _autoopenangle)
        (`self.UpdateDoorState` :!label _label_2)
        (else
          (`KismetSystemLibrary.Delay` 0.001 :!label _label_3)
          (`self.CheckDoorRotation`)))
      (elif (< _degree (* _autoopenangle -1.0))
        (goto _label_2)
        (else
          (goto _label_3))))
    (else
      (goto _label_3))))

(event `LockedEvent`
  ;[0.01 0.01 0.01] Locked
  (if (`|EnumEquality` (`self.DoorState`) "NewEnumerator0")
    (`|ExecutionSequence`
      (:`then_0`
        (if (not (`TimelineComponent.IsPlaying` (`self.Locked_TL`)))
          (bind (_direction _alpha) (`Timeline|Locked_TL` :!via `PlayFromStart` :!label _label_4)
            (:`Update`
              (`SceneComponent.K2_SetRelativeRotation` (`self.Door`) (`KismetMathLibrary.RLerp` (`SceneComponent.RelativeRotation` (`self.Door`)) (`KismetMathLibrary.MakeRotator` 0.0 0.0 _alpha) _alpha) false false)))
          (else
            (goto _label_4 :!via `Reverse`))))
      (:`then_1`
        (bind _returnvalue (`GameplayStatics.SpawnSoundAtLocation` (`self.LockedSound`) (`self.K2_GetActorLocation`) (struct) 1.0 1.0 0.0 null null))
        (`ActorComponent.SetActive` _returnvalue true (`AudioComponent.IsPlaying` _returnvalue))))))

(event `TriggerPhysicsSound`
  (bind _door (`self.Door`))
  ;[0.01 0.01 0.01] PhysicsSoundPlayer
  (if (`SceneComponent.IsSimulatingPhysics` _door "None")
    (if (> (`KismetMathLibrary.VSize` (`SceneComponent.GetComponentVelocity` _door)) 0.0)
      (`/Engine/EditorBlueprintResources/StandardMacros.DoOnce` false :!label _label_5
        (:`Completed`
          (`self.ActivatePhysicsSound`)))
      (else
        (`self.ClearPhysicsSound`)))))

(event `ResetPhysics Sound`
  ;[0.01 0.01 0.01] PhysicsSoundPlayer
  (goto _label_5 :!via `Reset`))

(event `self.AutoCloseCollision.OnComponentEndOverlap`
  (params (OverlappedComponent :type "PrimitiveComponent Object Reference") (OtherActor :type "Actor Object Reference") (OtherComp :type "PrimitiveComponent Object Reference") (OtherBodyIndex :type Integer))
  ;[0.01 0.01 0.01] Auto Close
  (if (== OtherActor (`GameplayStatics.GetPlayerCharacter` 0))
    (`self.ForceClose`)))

(event `SetLockState`
  (params (DoorLockType :type "/Game/TestV2/Blueprints/Enums/E_DoorLockTypes Enum" :default "NewEnumerator0"))
  ;[0.01 0.01 0.01] Call this event to lock or unlock doors.
  (bind _output_get (set `self.DoorLockType` DoorLockType))
  (switch `/Game/TestV2/Blueprints/Enums/E_DoorLockTypes` _output_get) ; Add what you want to happen when unlocked here - such as a sound effect.
)

(event `ForceOpen`
  ;[0.01 0.01 0.01] ForceOpenEvent
  (set `self.DoorLockType` "NewEnumerator0")
  (`self.RotateDoor` 25.0)
  (bind _output_get (set `self.DoorState` "NewEnumerator1"))
  (switch `/Game/TestV2/Blueprints/Enums/E_DoorStates` _output_get
    (:`NewEnumerator1`
      (`KismetSystemLibrary.Delay` 0.1)
      (`self.StopDoor_TL`)
      (`PrimitiveComponent.SetSimulatePhysics` (`self.Door`) true)
      (`self.CheckDoorRotation`))))

(fn `CalculateOpenDirection`
  (returns (Direction :type "Float (double-precision)"))
  (return (`KismetMathLibrary.SelectFloat` 1.0 -1.0 (> (`KismetMathLibrary.Dot_VectorVector` (`self.GetActorForwardVector` (`GameplayStatics.GetPlayerCharacter` 0)) (`SceneComponent.GetForwardVector` (`self.OpenDirection`))) 0.0))))

(fn `CalculatePhysicsDoorDegree`
  (returns (Degree :type "Float (single-precision)"))
  (return (.yaw (.rotation (`KismetMathLibrary.MakeRelativeTransform` (`SceneComponent.K2_GetComponentToWorld` (`self.Door`)) (`SceneComponent.K2_GetComponentToWorld` (`self.DoorFrame`)))))))

(fn `ForceClose`
  (switch `/Game/TestV2/Blueprints/Enums/E_DoorStates` (`self.DoorState`)
    (:`NewEnumerator1`
      (`self.ClearPhysicsSound`)
      (`self.ReparentDoor`))
    (:`NewEnumerator2`
      _))
  (`PrimitiveComponent.SetSimulatePhysics` (`self.Door`) false)
  (`self.RotateDoor` 0.0)
  (set `self.DoorState` "NewEnumerator0")
  (bind _returnvalue (`GameplayStatics.SpawnSoundAtLocation` (`self.SoftCloseSound`) (`self.K2_GetActorLocation`) (struct) 1.0 1.0 0.0 null null))
  (`ActorComponent.SetActive` _returnvalue true (`AudioComponent.IsPlaying` _returnvalue)))

(fn `ReparentDoor`
  (set `self.WorldRotation` (`SceneComponent.K2_GetComponentRotation` (`self.Door`)))
  (`PrimitiveComponent.SetSimulatePhysics` (`self.Door`) false)
  (`SceneComponent.K2_AttachToComponent` (`self.Door`) (`self.DoorFrame`) "None" "SnapToTarget" "KeepWorld" "SnapToTarget" true)
  (`SceneComponent.K2_SetRelativeLocation` (`self.Door`) (0.0 45.0 5.0) false false))

(fn `UpdateDoorState`
  (returns (`Door State` :type "/Game/TestV2/Blueprints/Enums/E_DoorStates Enum"))
  (bind _door_tl (`self.Door_TL`))
  (switch `/Game/TestV2/Blueprints/Enums/E_DoorStates` (`self.DoorState`)
    (:`NewEnumerator0`
      (if (not (`self.StateActive`))
        (`TimelineComponent.SetPlayRate` _door_tl 0.6)
        (`self.RotateDoor` 25.0)
        (bind _output_get (set `self.DoorState` "NewEnumerator1"))
        (return _output_get)))
    (:`NewEnumerator1`
      (`TimelineComponent.SetPlayRate` _door_tl 1.0)
      (`self.ClearPhysicsSound`)
      (`self.ReparentDoor`)
      (`self.RotateDoor` 95.0)
      (bind _output_get_2 (set `self.DoorState` "NewEnumerator2"))
      (return _output_get_2))
    (:`NewEnumerator2`
      (`TimelineComponent.SetPlayRate` _door_tl 0.5)
      (`PrimitiveComponent.SetSimulatePhysics` (`self.Door`) false)
      (`self.RotateDoor` 0.0)
      (bind _output_get_3 (set `self.DoorState` "NewEnumerator0"))
      (bind _returnvalue (`GameplayStatics.SpawnSoundAtLocation` (`self.CloseSound`) (`self.K2_GetActorLocation`) (struct) 1.0 1.0 0.0 null null))
      (`ActorComponent.SetActive` _returnvalue true (`AudioComponent.IsPlaying` _returnvalue))
      (return _output_get_3))))

(fn `UserConstructionScript`)