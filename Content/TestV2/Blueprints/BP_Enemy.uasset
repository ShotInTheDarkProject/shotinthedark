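; BP_Enemy is an AI enemy that roams at random and moves toward pawns it sees.
; RandomRoam repeatedly moves it to random reachable points nearby, while PawnSensing redirects it to the seen pawn and resumes roaming after a retriggerable delay.
; BeginPlay starts roaming, plays a sound at its location, and runs a separate delayed loop of move orders to its own current location.
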(event `self.PawnSensing.OnSeePawn`
  (params (Pawn :type "Pawn Object Reference"))
  ;[1 1 1] AI CHASE
  (`|ExecutionSequence`
    (:`then_0`
      (`|AIMoveTo` self (0.0 0.0 0.0) Pawn))
    (:`then_1`
      (`KismetSystemLibrary.RetriggerableDelay` 1.0)
      (`self.Random Roam`))))

(event `Random Roam`
  (`|AIMoveTo` null (`NavigationSystemV1.K2_GetRandomReachablePointInRadius` (`self.K2_GetActorLocation`) 1500.0 null null) null
    (:`OnSuccess`
      (`self.Random Roam`))))

(event `self.ReceiveBeginPlay`
  (`self.Random Roam`)
  (`|ExecutionSequence`
    (:`then_0`
      (`|AIMoveTo` self (`self.K2_GetActorLocation`) null :!label _label
        (:`OnSuccess`
          (`KismetSystemLibrary.Delay` 2.0)
          (goto _label))))
    (:`then_1`
      (`GameplayStatics.PlaySoundAtLocation` "/Game/TestV2/Demo/Enemy/EnemyCue.EnemyCue" (`self.K2_GetActorLocation`) (struct) 1.0 1.0 0.0 null null null null))))

(fn `UserConstructionScript`)