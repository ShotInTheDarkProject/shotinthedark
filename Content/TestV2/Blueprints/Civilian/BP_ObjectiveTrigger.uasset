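; Rescue-zone trigger that tracks civilian "cargo" and resolves victory or defeat for all players.
; Overlaps add or remove civilians from Rescued and post notifications, though NotifyAllPlayers returns after the first character; entering players see the count.
; Tick polls characters, switching to DefeatCamera once all are dead and faded.
; When all civilians are rescued, it fades players out as escaped, then switches to VictoryCamera and shows the pre-created victory menu.
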(event `self.ReceiveBeginPlay`
  (`|ExecutionSequence`
    (:`then_0`
      (bind _outactors (`GameplayStatics.GetAllActorsOfClass` "/Game/TestV2/Blueprints/Civilian/BP_Civilian.BP_Civilian_C"))
      (set `self.Civilians` _outactors))
    (:`then_1`
      (bind _returnvalue (`|CreateWidget` "/Game/TestV2/Blueprints/Menus/W_MenuVictory.W_MenuVictory_C" (`GameplayStatics.GetPlayerController` 0)))
      (bind _output_get (set `self.MenuWidgetVictory` _returnvalue))
      (`Widget.SetVisibility` _output_get "Hidden")
      (`UserWidget.AddToViewport` _output_get 0))))

(event `self.ReceiveActorBeginOverlap`
  (params (OtherActor :type "Actor Object Reference"))
  (bind _rescued (`self.Rescued`))
  (if (== (`GameplayStatics.GetObjectClass` OtherActor) "/Game/TestV2/Blueprints/Character/BP_FPHorrorCharacter.BP_FPHorrorCharacter_C")
    (bind _asbp_fphorror_character (cast `/Game/TestV2/Blueprints/Character/BP_FPHorrorCharacter` OtherActor))
    (`/Game/TestV2/Blueprints/Character/BP_FPHorrorCharacter.NotifyPlayer` _asbp_fphorror_character (`KismetTextLibrary.Conv_StringToText` (`KismetStringLibrary.Concat_StrStr` (`KismetStringLibrary.Concat_StrStr` (`KismetStringLibrary.Concat_StrStr` (`KismetStringLibrary.Conv_IntToString` (`KismetArrayLibrary.Array_Length` (`self.Rescued`))) "/") (`KismetStringLibrary.Conv_IntToString` (`KismetArrayLibrary.Array_Length` (`self.Civilians`)))) " CARGO RESCUED")) (struct :`G` 0.690196 :`B` 1.0 :`A` 1.0) 3.0)
    (elif (`KismetArrayLibrary.Array_Contains` (`self.Civilians`) OtherActor)
      (if (not (`KismetArrayLibrary.Array_Contains` _rescued OtherActor))
        (`KismetArrayLibrary.Array_Add` _rescued OtherActor)
        (`self.NotifyAllPlayers` "CARGO RESCUED!" (struct :`G` 0.690196 :`B` 1.0 :`A` 1.0) 1.0)
        (if (== (`KismetArrayLibrary.Array_Length` (`self.Rescued`)) (`KismetArrayLibrary.Array_Length` (`self.Civilians`)))
          (`self.NotifyAllPlayers` "ALL CARGO RESCUED!" (struct :`G` 0.690196 :`B` 1.0 :`A` 1.0) 5.0))))))

(event `self.ReceiveActorEndOverlap`
  (params (OtherActor :type "Actor Object Reference"))
  (bind _rescued (`self.Rescued`))
  (if (`KismetArrayLibrary.Array_Contains` _rescued OtherActor)
    (`KismetArrayLibrary.Array_RemoveItem` _rescued OtherActor)
    (`self.NotifyAllPlayers` "CARGO LOST!" (struct :`R` 1.0 :`G` 0.918963 :`A` 1.0) 1.0)))

(event `self.ReceiveTick`
  (params (DeltaSeconds :type "Float (single-precision)"))
  (`|ExecutionSequence`
    (:`then_0`
      (set `self.Deaths` 0)
      (bind _outactors (`GameplayStatics.GetAllActorsOfClass` "/Game/TestV2/Blueprints/Character/BP_FPHorrorCharacter.BP_FPHorrorCharacter_C"))
      (for _array_element _outactors
        (if (`/Game/TestV2/Blueprints/Character/BP_FPHorrorCharacter.Dead` _array_element)
          (if (>= (`/Game/TestV2/Blueprints/Character/BP_FPHorrorCharacter.TransitionValue` _array_element) 1.0)
            (`/Engine/EditorBlueprintResources/StandardMacros.IncrementInt` (`self.Deaths`)))))
      (if (== (`KismetArrayLibrary.Array_Length` _outactors) (`self.Deaths`))
        (for _array_element_2 _outactors
          (`PlayerController.SetViewTargetWithBlend` (`GameplayStatics.GetPlayerController` (`/Game/TestV2/Blueprints/Character/BP_FPHorrorCharacter.PlayerIndex` _array_element_2)) (`self.DefeatCamera`) 0.0 "VTBlend_Linear" 0.0 false)
          (`/Game/TestV2/Blueprints/Character/BP_FPHorrorCharacter.StartTransitionFade` :`self` _array_element_2 :`StartOpacity` 1.0 :`FadeInterval` 0.001))))
    (:`then_1`
      (set `self.Escapes` 0)
      (if (== (`KismetArrayLibrary.Array_Length` (`self.Rescued`)) (`KismetArrayLibrary.Array_Length` (`self.Civilians`)))
        (bind _outactors_2 (`GameplayStatics.GetAllActorsOfClass` "/Game/TestV2/Blueprints/Character/BP_FPHorrorCharacter.BP_FPHorrorCharacter_C"))
        (for _array_element_3 _outactors_2
          (if (`/Game/TestV2/Blueprints/Character/BP_FPHorrorCharacter.Escaped` _array_element_3)
            (if (>= (`/Game/TestV2/Blueprints/Character/BP_FPHorrorCharacter.TransitionValue` _array_element_3) 1.0)
              (`/Engine/EditorBlueprintResources/StandardMacros.IncrementInt` (`self.Escapes`)))
            (else
              (`/Game/TestV2/Blueprints/Character/BP_FPHorrorCharacter.StartTransitionFade` :`self` _array_element_3 :`TargetOpacity` 1.0 :`FadeInterval` 0.01)
              (set `/Game/TestV2/Blueprints/Character/BP_FPHorrorCharacter.Escaped` true _array_element_3))))
        (if (== (`KismetArrayLibrary.Array_Length` _outactors_2) (`self.Escapes`))
          (for _array_element_4 _outactors_2
            (`PlayerController.SetViewTargetWithBlend` (`GameplayStatics.GetPlayerController` (`/Game/TestV2/Blueprints/Character/BP_FPHorrorCharacter.PlayerIndex` _array_element_4)) (`self.VictoryCamera`) 0.0 "VTBlend_Linear" 0.0 false)
            (`/Game/TestV2/Blueprints/Character/BP_FPHorrorCharacter.StartTransitionFade` :`self` _array_element_4 :`StartOpacity` 1.0 :`FadeInterval` 0.01)
            (`/Game/TestV2/Blueprints/Menus/W_MenuVictory.Show` (`self.MenuWidgetVictory`))))))))

(fn `NotifyAllPlayers`
  (params (Text :type Text) (Color :type "LinearColor Structure") (Time :type "Float (double-precision)"))
  (bind _outactors (`GameplayStatics.GetAllActorsOfClass` "/Game/TestV2/Blueprints/Character/BP_FPHorrorCharacter.BP_FPHorrorCharacter_C"))
  (for _array_element _outactors
    (`/Game/TestV2/Blueprints/Character/BP_FPHorrorCharacter.NotifyPlayer` _array_element Text Color Time)
    (return)))

(fn `UserConstructionScript`)