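; Critter enemy pawn that wanders the navmesh in loose boids-style swarms and is destroyed when damage drains its health.
; A repeating AI MoveTo loop gathers nearby critters, then heads along a velocity blending their averaged target velocities with separation from the nearest one.
; With too few neighbours or after a failed move, it steers toward a random reachable point instead.
; Pawn sensing events are empty stubs.
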(event `self.ReceiveAnyDamage`
  (params (Damage :type "Float (single-precision)") (DamageType :type "DamageType Object Reference") (InstigatedBy :type "Controller Object Reference") (DamageCauser :type "Actor Object Reference"))
  (bind _output_get (set `self.Health` (`KismetMathLibrary.FClamp` (- (`self.Health`) Damage) 0.0 100.0)))
  (if (== _output_get 0.0)
    (`self.K2_DestroyActor`)))

(event `Detect Swarm`
  ;[1 1 1] Reset swarm
  (set `self.Swarm` (`|MakeArray`))
  ;[1 1 1] Loop through all Critter enemies
  (bind _outactors (`GameplayStatics.GetAllActorsOfClass` "BP_Enemy_Critter_C"))
  (for _array_element _outactors
    ;[1 1 1] Add to swarm if nearby
    (if (== _array_element self)
      _
      (elif (<= (`KismetMathLibrary.Vector_Distance` (`self.K2_GetActorLocation` self) (`self.K2_GetActorLocation` _array_element)) (`self.BoidsDetectRadius`))
        (`KismetArrayLibrary.Array_Add` (`self.Swarm`) _array_element)))))

(event `Random Wander`
  (bind _returnvalue (`self.K2_GetActorLocation`))
  ;[1 1 1] Wander randomly
  (set `self.BoidsTargetVelocity` (+ (* (`self.BoidsTargetVelocity`) (- 0.25 (`self.BoidsSteer`))) (`KismetMathLibrary.GetDirectionUnitVector` _returnvalue (`NavigationSystemV1.K2_GetRandomReachablePointInRadius` _returnvalue (`self.WanderRadius`) null null)))))

(event `Swarm Wander`
  ;[1 1 1] Detect if alone or in group
  (`self.Detect Swarm`)
  (if (> (`KismetArrayLibrary.Array_Length` (`self.Swarm`)) 1)
    ;[1 1 1] Follow swarm
    (bind _velocity (`self.BoidsVelocity` (`self.Swarm`)))
    (set `self.BoidsTargetVelocity` _velocity)
    (else
      (`self.Random Wander`))))

(event `self.ReceiveBeginPlay`
  (`self.Swarm Wander` :!label _label)
  (`|AIMoveTo` self (+ (`self.K2_GetActorLocation`) (* (`self.BoidsTargetVelocity`) (`self.BoidsSpeed`))) null 3.0 :!label _label_2
    (:`then`
      (`KismetSystemLibrary.Delay` (`self.WanderDuration`))
      (goto _label))
    (:`OnFail`
      (`self.Random Wander`)
      (goto _label_2))))

(event `self.PawnSensing.OnHearNoise`
  (params (Instigator :type "Pawn Object Reference") (Location :type "Vector Structure (by ref)") (Volume :type "Float (single-precision)")))

(event `self.PawnSensing.OnSeePawn`
  (params (Pawn :type "Pawn Object Reference")))

(fn `BoidsVelocity`
  (params (Swarm :type "Array of /Game/TestV2/Blueprints/Enemy/BP_Enemy_Critter Object Reference"))
  (returns (Velocity :type "Vector Structure"))
  (locals (Average :type "Vector Structure"))
  (bind _returnvalue (`self.K2_GetActorLocation`))
  ;[1 1 1] Calculate the average direction of all swarm members
  (for _array_element Swarm
    (set `local.Average` (+ (`/Game/TestV2/Blueprints/Enemy/BP_Enemy_Critter.BoidsTargetVelocity` _array_element) (`local.Average`))))
  (return (+ (`KismetMathLibrary.GetDirectionUnitVector` (`self.K2_GetActorLocation` _array_element) (/ (`local.Average`) (`KismetArrayLibrary.Array_Length` Swarm))) (* (`KismetMathLibrary.GetDirectionUnitVector` (`self.K2_GetActorLocation` (`.ReturnValue` (`GameplayStatics.FindNearestActor` _returnvalue Swarm))) _returnvalue) (`self.BoidsSteer`)))))

(fn `UserConstructionScript`)