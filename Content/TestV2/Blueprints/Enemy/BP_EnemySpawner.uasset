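; Enemy spawner actor that keeps the number of BP_Enemy_Critter actors in the level topped up to a Desired count.
; Every Tick it counts all critters and, if short, spawns one at its location plus SpawnOffset.
; The SpawnTime Delay trails the spawn with nothing after it, so it does not throttle spawning.
; NotifyAllPlayers, not called here, sends a colored timed message but returns after the first BP_FPHorrorCharacter.
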(event `self.ReceiveTick`
  (params (DeltaSeconds :type "Float (single-precision)"))
  (bind _outactors (`GameplayStatics.GetAllActorsOfClass` "/Game/TestV2/Blueprints/Enemy/Critter/BP_Enemy_Critter.BP_Enemy_Critter_C"))
  (if (< (`KismetArrayLibrary.Array_Length` _outactors) (`self.Desired`))
    (`|SpawnActorFromClass` "/Game/TestV2/Blueprints/Enemy/Critter/BP_Enemy_Critter.BP_Enemy_Critter_C" (`KismetMathLibrary.Conv_VectorToTransform` (+ (`self.K2_GetActorLocation`) (`self.SpawnOffset`))) "Undefined" "MultiplyWithRoot" null null)
    (`KismetSystemLibrary.Delay` (`self.SpawnTime`))))

(fn `NotifyAllPlayers`
  (params (Text :type Text) (Color :type "LinearColor Structure") (Time :type "Float (double-precision)"))
  (bind _outactors (`GameplayStatics.GetAllActorsOfClass` "/Game/TestV2/Blueprints/Character/BP_FPHorrorCharacter.BP_FPHorrorCharacter_C"))
  (for _array_element _outactors
    (`/Game/TestV2/Blueprints/Character/BP_FPHorrorCharacter.NotifyPlayer` _array_element Text Color Time)
    (return)))

(fn `UserConstructionScript`)