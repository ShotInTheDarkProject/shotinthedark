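; BP_Fan_Vent is an environmental fan vent that spins and can be backlit.
; On BeginPlay it sets the light color and applies its Powered state through the Switch function.
; Switch stores the Powered value and, for backlit vents, toggles the light's visibility to match.
; While powered, Tick rotates the fan around yaw at FanSpeed each frame, without scaling by delta time.
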(event `self.ReceiveBeginPlay`
  (`|ExecutionSequence`
    (:`then_0`
      (`LightComponent.SetLightColor` (`self.Light`) (`self.LightColor`) true))
    (:`then_1`
      (`self.Switch` (`self.Powered`)))))

(event `self.ReceiveTick`
  (params (DeltaSeconds :type "Float (single-precision)"))
  (if (`self.Powered`)
    (`SceneComponent.K2_AddLocalRotation` (`self.Fan`) (`KismetMathLibrary.MakeRotator` 0.0 0.0 (`self.FanSpeed`)) false false)))

(fn `Switch`
  (params (Powered :type Boolean))
  (bind _output_get (set `self.Powered` Powered))
  (if (`self.Backlit`)
    (`SceneComponent.SetVisibility` (`self.Light`) _output_get false)))

(fn `UserConstructionScript`)